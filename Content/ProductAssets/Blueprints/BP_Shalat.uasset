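; Actor that demonstrates shalat (Islamic prayer) on a skeletal mesh with synced recitation audio, either as a full two-rakaat sequence or individual movements.
; BeginPlay creates the action-button widget and binds its SetAnimation event, whose index picks a MultiGate branch: full prayer, takbir, rukuk, sujud or tahiyat.
; Branches chain sound and animation calls with hand-timed Delays, then fire a ResetStateAction dispatcher that resets the gate.
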(event `self.ReceiveBeginPlay`
  (bind _actionbuttoncharacter (`self.CharacterActionHUD`))
  ;[1 1 1] Change and Play Animation
  (add `/Game/ProductAssets/Blueprints/WidgetBlueprint/WBP_CharacterShalatActionButton.SetAnimation` _actionbuttoncharacter (delegate `SetAnimation`)))

(event `SetAnimation`
  (params (Index :type Integer))
  ;[1 1 1] Change and Play Animation
  (add `self.ResetStateAction` (delegate `ResetStateAction_Event`))
  (`|MultiGate` false false Index :!label _label
    (:`Out 0`
      ;[1 1 1] Shalat Full
      (`self.PlayShalatAudio` "/Game/ProductAssets/Media/MediaSource/MS_AllahuAkbar.MS_AllahuAkbar")
      (`self.PlayPartOfShalatAnimation` "/Game/ProductAssets/Animations/SkeletalMeshAnimation/AnimationSequence/Partial/AS_02_Takbir.AS_02_Takbir")
      (`KismetSystemLibrary.Delay` 2.5)
      (`self.PlayShalatAudio` "/Game/ProductAssets/Media/MediaSource/MS_Doa_Iftitah.MS_Doa_Iftitah")
      (`KismetSystemLibrary.Delay` 30.0)
      (`self.PlayShalatAudio` "/Game/ProductAssets/Media/MediaSource/MS_Doa_Al_Fatihah.MS_Doa_Al_Fatihah")
      (`KismetSystemLibrary.Delay` 36.0)
      (`self.PlayShalatAudio` "/Game/ProductAssets/Media/MediaSource/MS_Surat_AnNas.MS_Surat_AnNas")
      (`KismetSystemLibrary.Delay` 22.0)
      (`self.PlayShalatAudio` "/Game/ProductAssets/Media/MediaSource/MS_Rukuk.MS_Rukuk")
      (`self.PlayPartOfShalatAnimation` "/Game/ProductAssets/Animations/SkeletalMeshAnimation/AnimationSequence/Partial/AS_03_Start_Rukuk.AS_03_Start_Rukuk")
      (`KismetSystemLibrary.Delay` 13.0)
      (`self.PlayShalatAudio` "/Game/ProductAssets/Media/MediaSource/MS_After_Rukuk.MS_After_Rukuk")
      (`self.PlayPartOfShalatAnimation` "/Game/ProductAssets/Animations/SkeletalMeshAnimation/AnimationSequence/Partial/AS_04_Finish_Rukuk.AS_04_Finish_Rukuk")
      (`KismetSystemLibrary.Delay` 2.94)
      (`self.PlayShalatAudio` "/Game/ProductAssets/Media/MediaSource/MS_RabbanaLakalhamdu.MS_RabbanaLakalhamdu")
      (`KismetSystemLibrary.Delay` 8.0)
      (`self.PlayShalatAudio` "/Game/ProductAssets/Media/MediaSource/MS_AllahuAkbar.MS_AllahuAkbar")
      (`self.PlayPartOfShalatAnimation` "/Game/ProductAssets/Animations/SkeletalMeshAnimation/AnimationSequence/Partial/AS_05_Start_Sujud_After_Rukuk.AS_05_Start_Sujud_After_Rukuk")
      (`KismetSystemLibrary.Delay` 2.0)
      (`self.PlayShalatAudio` "/Game/ProductAssets/Media/MediaSource/MS_Bacaan_Sujud.MS_Bacaan_Sujud")
      (`KismetSystemLibrary.Delay` 10.0)
      (`self.PlayShalatAudio` "/Game/ProductAssets/Media/MediaSource/MS_Takbir.MS_Takbir")
      (`self.PlayPartOfShalatAnimation` "/Game/ProductAssets/Animations/SkeletalMeshAnimation/AnimationSequence/Partial/AS_06_After_Sujud.AS_06_After_Sujud")
      (`KismetSystemLibrary.Delay` 1.73)
      (`self.PlayShalatAudio` "/Game/ProductAssets/Media/MediaSource/MS_Robirfirli.MS_Robirfirli")
      (`KismetSystemLibrary.Delay` 9.35)
      (`self.PlayShalatAudio` "/Game/ProductAssets/Media/MediaSource/MS_Takbir.MS_Takbir")
      (`self.PlayPartOfShalatAnimation` "/Game/ProductAssets/Animations/SkeletalMeshAnimation/AnimationSequence/Partial/AS_07_Start_Second_Sujud.AS_07_Start_Second_Sujud")
      (`KismetSystemLibrary.Delay` 1.73)
      (`self.PlayShalatAudio` "/Game/ProductAssets/Media/MediaSource/MS_Bacaan_Sujud.MS_Bacaan_Sujud")
      (`KismetSystemLibrary.Delay` 10.0)
      (`self.PlayShalatAudio` "/Game/ProductAssets/Media/MediaSource/MS_AllahuAkbar.MS_AllahuAkbar")
      (`self.PlayPartOfShalatAnimation` "/Game/ProductAssets/Animations/SkeletalMeshAnimation/AnimationSequence/Partial/AS_08_Stand_After_Second_Sujud.AS_08_Stand_After_Second_Sujud")
      (`KismetSystemLibrary.Delay` 2.0)
      (`self.PlayShalatAudio` "/Game/ProductAssets/Media/MediaSource/MS_Doa_Al_Fatihah.MS_Doa_Al_Fatihah")
      (`KismetSystemLibrary.Delay` 35.1)
      (`self.PlayShalatAudio` "/Game/ProductAssets/Media/MediaSource/MS_Surat_Al_Ikhlas.MS_Surat_Al_Ikhlas")
      (`KismetSystemLibrary.Delay` 16.6)
      (`self.PlayShalatAudio` "/Game/ProductAssets/Media/MediaSource/MS_Rukuk.MS_Rukuk")
      (`self.PlayPartOfShalatAnimation` "/Game/ProductAssets/Animations/SkeletalMeshAnimation/AnimationSequence/Partial/AS_09_Start_Second_Rukuk.AS_09_Start_Second_Rukuk")
      (`KismetSystemLibrary.Delay` 13.0)
      (`self.PlayShalatAudio` "/Game/ProductAssets/Media/MediaSource/MS_After_Rukuk.MS_After_Rukuk")
      (`self.PlayPartOfShalatAnimation` "/Game/ProductAssets/Animations/SkeletalMeshAnimation/AnimationSequence/Partial/AS_10_After_Second_Rukuk.AS_10_After_Second_Rukuk")
      (`KismetSystemLibrary.Delay` 2.94)
      (`self.PlayShalatAudio` "/Game/ProductAssets/Media/MediaSource/MS_RabbanaLakalhamdu.MS_RabbanaLakalhamdu")
      (`KismetSystemLibrary.Delay` 8.0)
      (`self.PlayShalatAudio` "/Game/ProductAssets/Media/MediaSource/MS_AllahuAkbar.MS_AllahuAkbar")
      (`self.PlayPartOfShalatAnimation` "/Game/ProductAssets/Animations/SkeletalMeshAnimation/AnimationSequence/Partial/AS_11_Start_Third_Sujud_After_Second_Rukuk.AS_11_Start_Third_Sujud_After_Second_Rukuk")
      (`KismetSystemLibrary.Delay` 2.0)
      (`self.PlayShalatAudio` "/Game/ProductAssets/Media/MediaSource/MS_Bacaan_Sujud.MS_Bacaan_Sujud")
      (`KismetSystemLibrary.Delay` 10.0)
      (`self.PlayShalatAudio` "/Game/ProductAssets/Media/MediaSource/MS_Takbir.MS_Takbir")
      (`self.PlayPartOfShalatAnimation` "/Game/ProductAssets/Animations/SkeletalMeshAnimation/AnimationSequence/Partial/AS_12_After_Third_Sujud.AS_12_After_Third_Sujud")
      (`KismetSystemLibrary.Delay` 1.73)
      (`self.PlayShalatAudio` "/Game/ProductAssets/Media/MediaSource/MS_Robirfirli.MS_Robirfirli")
      (`KismetSystemLibrary.Delay` 9.35)
      (`self.PlayShalatAudio` "/Game/ProductAssets/Media/MediaSource/MS_Takbir.MS_Takbir")
      (`self.PlayPartOfShalatAnimation` "/Game/ProductAssets/Animations/SkeletalMeshAnimation/AnimationSequence/Partial/AS_13_Start_Fourth_Sujud.AS_13_Start_Fourth_Sujud")
      (`KismetSystemLibrary.Delay` 1.73)
      (`self.PlayShalatAudio` "/Game/ProductAssets/Media/MediaSource/MS_Bacaan_Sujud.MS_Bacaan_Sujud")
      (`KismetSystemLibrary.Delay` 10.0)
      (`self.PlayShalatAudio` "/Game/ProductAssets/Media/MediaSource/MS_AtahiyatAkhir.MS_AtahiyatAkhir")
      (`self.PlayPartOfShalatAnimation` "/Game/ProductAssets/Animations/SkeletalMeshAnimation/AnimationSequence/Partial/AS_14_After_Fourth_Sujud.AS_14_After_Fourth_Sujud")
      (`KismetSystemLibrary.Delay` 17.0)
      (`self.PlayPartOfShalatAnimation` "/Game/ProductAssets/Animations/SkeletalMeshAnimation/AnimationSequence/Partial/AS_15_Start_Pointing.AS_15_Start_Pointing")
      (`KismetSystemLibrary.Delay` 33.0)
      (`self.PlayPartOfShalatAnimation` "/Game/ProductAssets/Animations/SkeletalMeshAnimation/AnimationSequence/Partial/AS_15_Start_Pointing.AS_15_Start_Pointing")
      (`KismetSystemLibrary.Delay` 1.0)
      (`self.PlayPartOfShalatAnimation` "/Game/ProductAssets/Animations/SkeletalMeshAnimation/AnimationSequence/Partial/AS_17_Salam.AS_17_Salam")
      (`self.ResetStateAction`))
    (:`Out 1`
      ;[1 1 1] Takbiratul Irham
      (`self.PlayShalatAudio` "/Game/ProductAssets/Media/MediaSource/MS_AllahuAkbar.MS_AllahuAkbar")
      (`self.PlayPartOfShalatAnimation` "/Game/ProductAssets/Animations/SkeletalMeshAnimation/AnimationSequence/Partial/AS_02_Takbir.AS_02_Takbir")
      (`self.ResetStateAction`))
    (:`Out 2`
      ;[1 1 1] Rukuk
      (`self.PlayShalatAudio` "/Game/ProductAssets/Media/MediaSource/MS_Rukuk.MS_Rukuk")
      (`self.PlayPartOfShalatAnimation` "/Game/ProductAssets/Animations/SkeletalMeshAnimation/AnimationSequence/Partial/AS_03_Start_Rukuk.AS_03_Start_Rukuk")
      (`self.ResetStateAction`))
    (:`Out 3`
      ;[1 1 1] Sujud
      (`self.PlayShalatAudio` "/Game/ProductAssets/Media/MediaSource/MS_Sujud.MS_Sujud")
      (`self.PlayPartOfShalatAnimation` "/Game/ProductAssets/Animations/SkeletalMeshAnimation/AnimationSequence/Partial/AS_05_Start_Sujud_After_Rukuk.AS_05_Start_Sujud_After_Rukuk")
      (`self.ResetStateAction`))
    (:`Out 4`
      ;[1 1 1] Takhiyat
      (`self.PlayShalatAudio` "/Game/ProductAssets/Media/MediaSource/MS_AtahiyatAkhir.MS_AtahiyatAkhir")
      (`self.PlayPartOfShalatAnimation` "/Game/ProductAssets/Animations/SkeletalMeshAnimation/AnimationSequence/Partial/AS_14_After_Fourth_Sujud.AS_14_After_Fourth_Sujud")
      (`KismetSystemLibrary.Delay` 17.0)
      (`self.PlayPartOfShalatAnimation` "/Game/ProductAssets/Animations/SkeletalMeshAnimation/AnimationSequence/Partial/AS_15_Start_Pointing.AS_15_Start_Pointing")
      (`KismetSystemLibrary.Delay` 33.0)
      (`self.PlayPartOfShalatAnimation` "/Game/ProductAssets/Animations/SkeletalMeshAnimation/AnimationSequence/Partial/AS_15_Start_Pointing.AS_15_Start_Pointing")
      (`KismetSystemLibrary.Delay` 1.0)
      (`self.PlayPartOfShalatAnimation` "/Game/ProductAssets/Animations/SkeletalMeshAnimation/AnimationSequence/Partial/AS_17_Salam.AS_17_Salam")
      (`self.ResetStateAction`))))

(event `ResetStateAction_Event`
  ;[1 1 1] Change and Play Animation
  (goto _label :!via `Reset`))

(event `self.ReceiveTick`
  (params (DeltaSeconds :type "Float (single-precision)")))

(fn `CharacterActionHUD`
  (returns (ActionButtonCharacter :type "/Game/ProductAssets/Blueprints/WidgetBlueprint/WBP_CharacterShalatActionButton Object Reference"))
  (bind _returnvalue (`|CreateWidget` "/Game/ProductAssets/Blueprints/WidgetBlueprint/WBP_CharacterShalatActionButton.WBP_CharacterShalatActionButton_C"))
  (bind _output_get (set `self.WBPCharacterAction` _returnvalue))
  (`UserWidget.AddToViewport` _output_get 0)
  (return _output_get))

(fn `PlayAnimation`
  (params (AnimationIndex :type Integer))
  (`SkeletalMeshComponent.PlayAnimation` (`self.SkeletalMeshComponent`) (`|GetArrayItem` (`self.Animations`) AnimationIndex) false))

(fn `PlayPartOfShalatAnimation`
  (params (AnimToPlay :type "AnimSequence Object Reference"))
  (`SkeletalMeshComponent.PlayAnimation` (`self.SkeletalMeshComponent`) AnimToPlay false))

(fn `PlayShalatAudio`
  (params (Sound :type "SoundBase Object Reference"))
  (bind _audio (`self.Audio`))
  (`AudioComponent.SetSound` _audio Sound)
  (`AudioComponent.Play` _audio 0.0))

(fn `UserConstructionScript`)